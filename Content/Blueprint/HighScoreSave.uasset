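; HighScoreSave holds an array of score entries, with functions to search and reorder that high score table.
; FindLowestScore and FindHighestScore scan the array and return an entry with its index.
; Despite its name, FindHighestScore also selects the lowest score, as its comparison is inverted.
; SortSaveData repeatedly moves FindHighestScore's pick into a temporary array and copies that back, so the resulting order is ascending.
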(fn FindLowestScore
  (for (_array_element _array_index) (Variables|Default|GetSaveStruct)
    (if (== _array_index 0)
      (LocalVariables|SetLowestScore (.score _array_element))
      (LocalVariables|SetLowestIndex _array_index)
      (elif (< (.score _array_element) (LocalVariables|GetLowestScore))
        (LocalVariables|SetLowestScore (.score _array_element))
        (LocalVariables|SetLowestIndex _array_index))))
  (return (Utilities|Array|Get(acopy) (Variables|Default|GetSaveStruct) (LocalVariables|GetLowestIndex)) (LocalVariables|GetLowestIndex)))

(fn FindHighestScore
  (for (_array_element _array_index) (Variables|Default|GetSaveStruct)
    (if (== _array_index 0)
      (LocalVariables|SetHighestScore (.score _array_element))
      (LocalVariables|SetHighestIndex _array_index)
      (elif (> (LocalVariables|GetHighestScore) (.score _array_element))
        (LocalVariables|SetHighestScore (.score _array_element))
        (LocalVariables|SetHighestIndex _array_index))))
  (return (Utilities|Array|Get(acopy) (Variables|Default|GetSaveStruct) (LocalVariables|GetHighestIndex)) (LocalVariables|GetHighestIndex)))

(fn SortSaveData
  (while (> (Utilities|Array|Length (Variables|Default|GetSaveStruct)) 0)
    (bind (_highestscorestruct _highestscoreindex) (CallFunction|FindHighestScore))
    (Utilities|Array|Add (LocalVariables|GetTempSaveStruct) _highestscorestruct)
    (Utilities|Array|RemoveIndex (Variables|Default|GetSaveStruct) _highestscoreindex))
  (Variables|Default|SetSaveStruct (LocalVariables|GetTempSaveStruct)))